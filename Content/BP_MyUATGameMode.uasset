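; Game mode providing level flow (restart, next level, main menu), pause, quit, and saved main-volume handling.
; OpenNextLevel finds the current map by name in the Level array from index 1, opening the following entry or falling back to MainMenu.
; BeginPlay loads the "Main" save slot and applies MainVolume through a sound mix override.
; SaveSaveGame writes MainVolume back, but the step restoring it on load is disconnected.
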(event `self.ReceiveBeginPlay`
  (`self.LoadSaveGame`)
  (`self.UpdateSound`))

(fn `LoadMainMenu`
  (`GameplayStatics.OpenLevelBySoftObjectPtr` "/Game/ThirdPerson/Maps/MainMenu.MainMenu"))

(fn `LoadSaveGame`
  (bind _returnvalue (`GameplayStatics.LoadGameFromSlot` "Main"))
  (bind _assave_game_data (cast `/Game/SaveSystem/SaveGameData` _returnvalue))
  (bind _output_get (set `self.SaveData` _assave_game_data)))

(fn `OpenNextLevel`
  (set `self.LevelToLoad` 0)
  (for _index (range 1 (+ (`KismetArrayLibrary.Array_LastIndex` (`self.Level`)) 1))
    (bind _returnvalue (`GameplayStatics.GetCurrentLevelName` true))
    (if (`KismetStringLibrary.EqualEqual_StrStr` _returnvalue (`KismetSystemLibrary.GetObjectName` (`|ConvertAsset` (`|GetArrayItem` (`self.Level`) _index))))
      (bind _output_get (set `self.LevelToLoad` (+ _index 1)))
      (if (`KismetMathLibrary.InRange_IntInt` _output_get 0 (`KismetArrayLibrary.Array_LastIndex` (`self.Level`)))
        (`GameplayStatics.OpenLevelBySoftObjectPtr` (`|GetArrayItem` (`self.Level`) (`self.LevelToLoad`)))
        (return)
        (else
          (`self.LoadMainMenu` :!label _label)))))
  (goto _label))

(fn `PauseGame`
  (`GameplayStatics.SetGamePaused` true))

(fn `QuitGame`
  (`KismetSystemLibrary.QuitGame` (`GameplayStatics.GetPlayerController` 0) "Quit")
  (return))

(fn `RestartLevel`
  (bind _returnvalue (`GameplayStatics.GetCurrentLevelName` true))
  (`GameplayStatics.OpenLevel` (`KismetStringLibrary.Conv_StringToName` _returnvalue))
  (return))

(fn `SaveSaveGame`
  (set `/Game/SaveSystem/SaveGameData.MainAudioVolume` (`self.MainVolume`) (`self.SaveData`))
  (`GameplayStatics.SaveGameToSlot` (`self.SaveData`) "Main"))

(fn `UpdateSound`
  (`GameplayStatics.SetSoundMixClassOverride` "/Game/Audio/Main_Mix.Main_Mix" "/Game/Audio/Main.Main" (`self.MainVolume`))
  (`GameplayStatics.PushSoundMixModifier` "/Game/Audio/Main_Mix.Main_Mix"))

(fn `UserConstructionScript`)