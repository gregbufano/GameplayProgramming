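; BP_UATEnemy is an AI enemy that spots the player, punches and can be stunned.
; Pawn sensing sets the CanSeePlayer blackboard key, which this file never clears.
; Attack starts a punch montage and sound and immediately damages player character 0, with no range or hit check.
; StunBegin sets the isStunned key, and a timer calls StunEnd to clear it.
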(event `self.PawnSensing.OnSeePawn`
  (params (Pawn :type "Pawn Object Reference"))
  ; Allow AI to see player and act on vision
  (cast `/Game/BP_MyUATCharacter` Pawn)
  (`BlackboardComponent.SetValueAsBool` (`AIBlueprintHelperLibrary.GetBlackboard` (`AIBlueprintHelperLibrary.GetAIController` self)) "CanSeePlayer" true))

(event `Attack`
  ; Logic for the AI to attack
  (`|PlayMontage` (`self.Mesh`) "/Game/Animation/Punching.Punching"
    (:`then`
      (`GameplayStatics.PlaySoundAtLocation` "/Game/Audio/Punch_Cue.Punch_Cue" (`self.K2_GetActorLocation`) (struct) 1.0 1.0 0.0 null null null null)
      (`GameplayStatics.ApplyDamage` (`GameplayStatics.GetPlayerCharacter` 0) 10.0))))

(event `StunBegin`
  ; Starting the stun
  (`BlackboardComponent.SetValueAsBool` (`AIBlueprintHelperLibrary.GetBlackboard` (`self.GetOwner`)) "isStunned" true)
  (`KismetSystemLibrary.PrintString` "Stun Starts")
  (`KismetSystemLibrary.K2_SetTimerDelegate` (delegate `StunEnd`) (`self.Time`) false false))

(event `StunEnd`
  ; Logic for ending stun after a certain amount of time
  (`BlackboardComponent.SetValueAsBool` (`AIBlueprintHelperLibrary.GetBlackboard` (`self.GetOwner`)) "isStunned" false)
  (`KismetSystemLibrary.PrintString` "Stun ends"))

(fn `UserConstructionScript`)