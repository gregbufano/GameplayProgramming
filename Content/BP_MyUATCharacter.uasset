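; BP_MyUATCharacter is a player character with health, a death sequence and an area stun ability.
; It adds a health widget on BeginPlay, and AnyDamage lowers Health, playing the Dying montage before destroying the actor; M applies test self-damage.
; The Stun input sphere-traces around the character and calls StunBegin on each BP_UATEnemy hit.
; Its cooldown is unfinished: StunCooldown only re-arms itself by timer, and the IsAbilityonCD branch is empty.
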(event `self.ReceiveBeginPlay`
  (bind _returnvalue (`|CreateWidget` "/Game/HealthUI/WHealth.WHealth_C" (`GameplayStatics.GetPlayerController` 0)))
  (`UserWidget.AddToViewport` _returnvalue 0))

(event `Key|M`
  (params (Key :type "Key Structure"))
  (:`Pressed`
    (`GameplayStatics.ApplyDamage` self 10.0)))

(event `self.ReceiveAnyDamage`
  (params (Damage :type "Float (single-precision)") (DamageType :type "DamageType Object Reference") (InstigatedBy :type "Controller Object Reference") (DamageCauser :type "Actor Object Reference"))
  ; Logic for enemy attack dealing damage
  (set `self.Health` (- (`self.Health`) Damage))
  (if (<= (`self.Health`) 0.0)
    (`KismetSystemLibrary.PrintString` "Death")
    (`|PlayMontage` (`self.Mesh`) "/Game/Animation/Dying.Dying"
      (:`then`
        (`KismetSystemLibrary.Delay` 2.0)
        (`self.K2_DestroyActor`)))
    (else
      (`KismetSystemLibrary.PrintString` (`KismetStringLibrary.Conv_DoubleToString` (`self.Health`))))))

(event `InputAction|Stun`
  (params (Key :type "Key Structure"))
  (bind _returnvalue (`self.K2_GetActorLocation`))
  ; Stun logic. Checks within a sphere for all actors hit by stun and activates enemy stun effect
  (:`Pressed`
    (bind (_outhits _returnvalue_2) (`KismetSystemLibrary.SphereTraceMultiForObjects` _returnvalue _returnvalue (`self.StunRadius`) (`self.StunObjectType`)))
    (if _returnvalue_2
      (for _array_element _outhits
        (bind _asbp_uatenemy (cast `/Game/AI/BP_UATEnemy` (`.HitActor` (`GameplayStatics.BreakHitResult` _array_element))))
        (`/Game/AI/BP_UATEnemy.StunBegin` _asbp_uatenemy)
        (`self.StunCooldown`)))))

(event `StunCooldown`
  ; Stun logic. Checks within a sphere for all actors hit by stun and activates enemy stun effect
  (`KismetSystemLibrary.K2_SetTimerDelegate` (delegate `StunCooldown`) (`self.StunAbilityCD`))
  (if (`self.isAbilityonCD`)
    _))

(fn `UserConstructionScript`)